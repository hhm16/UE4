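; Defense tower actor that automatically attacks nearby enemies and can be reloaded by the hero.
; A repeating sphere trace gathers EnemyCharacters in range, and EnemyDistanceToTower picks the closest as target.
; Attack yaws the weapon unless IsRangeAttack, plays the fire montage, spawns a targeted projectile on its notify and repeats after AttackInterval.
; Hero overlap shows ammo text and enables Reload input; overlapping Projectiles are destroyed.
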(event `self.ReceiveBeginPlay`
  (`KismetSystemLibrary.K2_SetTimerDelegate` (delegate `search_enemy`) 0.1)
  (`self.HideAmmoNum`)
  (`self.EnableInput` (`GameplayStatics.GetPlayerController` 0)))

(event `search_enemy`
  (bind _returnvalue (`self.K2_GetActorLocation`))
  (`KismetSystemLibrary.Delay` 0.05)
  (bind (_outhits _returnvalue_2) (`KismetSystemLibrary.SphereTraceMultiForObjects` :`Start` _returnvalue :`End` _returnvalue :`Radius` (`self.AttackRange`) :`ObjectTypes` (`|MakeArray` "ObjectTypeQuery3" :!type "EObjectTypeQuery Enum") :`DrawDebugType` "ForDuration"))
  (if _returnvalue_2
    (`KismetArrayLibrary.Array_Clear` (`self.searched_enemy_array`))
    (for _array_element _outhits
      (bind _asenemy_character (cast `/Game/Blueprints/EnemyCharacter` (`.HitActor` (`GameplayStatics.BreakHitResult` _array_element))))
      (`KismetArrayLibrary.Array_Add` (`self.searched_enemy_array`) _asenemy_character))
    (if (>= (`KismetArrayLibrary.Array_Length` (`self.searched_enemy_array`)) 1)
      (bind _hasenemy_ (`self.EnemyDistanceToTower`))
      (if _hasenemy_
        (`self.Attack`)
        (else
          (`self.search_enemy` :!label _label)))
      (else
        (goto _label)))
    (else
      (`self.search_enemy`))))

(event `Attack`
  (bind (_returnvalue_roll _returnvalue_pitch _returnvalue_yaw) (`KismetMathLibrary.BreakRotator` (`KismetMathLibrary.FindLookAtRotation` (`self.K2_GetActorLocation`) (`self.K2_GetActorLocation` (`self.EnemyToAttack`)))))
  (`self.EnemyToAttack`
    (:`then`
      (if (> (`self.ammoNum`) 0)
        (if (not (`self.isRangeAttack`))
          (`SceneComponent.K2_SetWorldRotation` (`self.TowerWeapon`) (`KismetMathLibrary.MakeRotator` 0.0 0.0 _returnvalue_yaw) false false))
        (if (>= (`KismetMathLibrary.VSize` (- (`self.K2_GetActorLocation`) (`self.K2_GetActorLocation` (`self.EnemyToAttack`)))) (`self.AttackRange`))
          (set `self.EnemyToAttack` null)
          (`self.search_enemy` :!label _label_2)
          (else
            (bind _enemytoattack (`self.EnemyToAttack`)
              (:`then`
                (`|PlayMontage` (`self.TowerWeapon`) (`self.FireMontage`)
                  (:`then`
                    (set `self.isAttacking` true)
                    (`/Engine/EditorBlueprintResources/StandardMacros.DecrementInt` (`self.ammoNum`)
                      (:`  `
                        (`TextRenderComponent.K2_SetText` (`self.TextRender_AmmoNum`) (`KismetTextLibrary.Conv_IntToText` (`self.ammoNum`))))))
                  (:`OnNotifyBegin`
                    (`|SpawnActorFromClass` "/Game/DefenseTower/Blueprints/TowerWeapon_Basic.TowerWeapon_Basic_C" (`SceneComponent.K2_GetComponentToWorld` (`self.Arrow`)) "Undefined" "OverrideRootScale" null _enemytoattack null)
                    (`KismetSystemLibrary.Delay` (`self.AttackInterval`))
                    (`/Engine/EditorBlueprintResources/StandardMacros.IsValid` (`self.EnemyToAttack`)
                      (:`Is Valid`
                        (`self.Attack`))
                      (:`Is Not Valid`
                        (set `self.isAttacking` false)
                        (`self.search_enemy`))))))
              (:`else`
                (goto _label_2)))))
        (else
          (`self.search_enemy`))))
    (:`else`)))

(event `DisplayAmmoNum`
  (`SceneComponent.SetVisibility` (`self.TextRender_Ammo`) true false)
  (`SceneComponent.SetVisibility` (`self.TextRender_AmmoNum`) true false))

(event `HideAmmoNum`
  (`SceneComponent.SetVisibility` (`self.TextRender_Ammo`) false false)
  (`SceneComponent.SetVisibility` (`self.TextRender_AmmoNum`) false false))

(event `self.HeroDetecter.OnComponentBeginOverlap`
  (params (OverlappedComponent :type "PrimitiveComponent Object Reference") (OtherActor :type "Actor Object Reference") (OtherComp :type "PrimitiveComponent Object Reference") (OtherBodyIndex :type Integer) (bFromSweep :type Boolean) (SweepResult :type "HitResult Structure (by ref)"))
  (cast `/Game/Blueprints/HeroCharacter` OtherActor)
  (`self.DisplayAmmoNum`)
  (set `self.canReloadNow` true))

(event `self.HeroDetecter.OnComponentEndOverlap`
  (params (OverlappedComponent :type "PrimitiveComponent Object Reference") (OtherActor :type "Actor Object Reference") (OtherComp :type "PrimitiveComponent Object Reference") (OtherBodyIndex :type Integer))
  (cast `/Game/Blueprints/HeroCharacter` OtherActor)
  (`self.HideAmmoNum`)
  (set `self.canReloadNow` false))

(event `InputAction|Reload`
  (params (Key :type "Key Structure"))
  (:`Pressed`
    (if (`self.canReloadNow`)
      (bind _output_get (set `self.ammoNum` 100))
      (`TextRenderComponent.K2_SetText` (`self.TextRender_AmmoNum`) (`KismetTextLibrary.Conv_IntToText` _output_get)))))

(event `self.ReceiveActorBeginOverlap`
  (params (OtherActor :type "Actor Object Reference"))
  (cast `/Game/Blueprints/Projectile` OtherActor)
  (`self.K2_DestroyActor` OtherActor))

(fn `EnemyDistanceToTower`
  (returns (`hasEnemy?` :type Boolean))
  (locals (EnemyDistanceRemember :type "Float (double-precision)" :default 99999.0) (NearestEnemyRemember :type "/Game/Blueprints/EnemyCharacter Object Reference"))
  (for _array_element (`self.searched_enemy_array`)
    (bind _returnvalue (`KismetMathLibrary.VSize` (- (`self.K2_GetActorLocation`) (`self.K2_GetActorLocation` _array_element))))
    (if (<= _returnvalue (`local.EnemyDistanceRemember`))
      (set `local.EnemyDistanceRemember` _returnvalue)
      (set `self.EnemyToAttack` _array_element)))
  (return (`KismetSystemLibrary.IsValid` (`self.EnemyToAttack`))))

(fn `UserConstructionScript`)