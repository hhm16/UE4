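; Boom is an explosive projectile actor in the DefenseTower game that bursts on impact or destroys itself after a fixed delay.
; On hit it spawns an explosion emitter, then sphere-traces pawns within ExplosionRange and spawns sparks on each EnemyCharacter, applying no damage here.
; It then destroys itself.
; Tick sets the same fixed rotation each frame, so it does not spin despite its comment.
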(event `self.ReceiveBeginPlay`
  ;[1 1 1] Destroys actor after either the projectile collides with an object or after 10 seconds
  (`KismetSystemLibrary.Delay` 15.0)
  (`self.K2_DestroyActor`))

(event `self.ReceiveHit`
  (params (MyComp :type "PrimitiveComponent Object Reference") (Other :type "Actor Object Reference") (OtherComp :type "PrimitiveComponent Object Reference") (bSelfMoved :type Boolean) (HitLocation :type "Vector Structure") (HitNormal :type "Vector Structure") (NormalImpulse :type "Vector Structure") (Hit :type "HitResult Structure (by ref)"))
  (bind _returnvalue (`self.K2_GetActorLocation`))
  ;[1 1 1] Event hit determines spawn location for impact effect
  (`GameplayStatics.SpawnEmitterAtLocation` "/Game/BeamsAndLazers/Particles/P_ExplosionWhite.P_ExplosionWhite" HitLocation (struct) (3.0 3.0 3.0))
  (bind _outhits (`KismetSystemLibrary.SphereTraceMultiForObjects` _returnvalue _returnvalue (`self.ExplosionRange`) (`|MakeArray` "ObjectTypeQuery3" :!type "EObjectTypeQuery Enum")))
  (for _array_element _outhits
    (bind _asenemy_character (cast `/Game/Blueprints/EnemyCharacter` (`.HitActor` (`GameplayStatics.BreakHitResult` _array_element))))
    (`GameplayStatics.SpawnEmitterAtLocation` "/Game/StarterContent/Particles/LaserSpark_R.LaserSpark_R" (`self.K2_GetActorLocation` _asenemy_character) (struct) (4.0 4.0 4.0)))
  (`self.K2_DestroyActor`))

(event `self.ReceiveTick`
  (params (DeltaSeconds :type "Float (single-precision)"))
  ;[1 1 1] Continually rotates actor per tick
  (`self.K2_SetActorRotation` (struct :`Pitch` 1.0 :`Yaw` 1.0)))

(fn `UserConstructionScript`)