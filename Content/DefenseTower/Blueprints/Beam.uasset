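; Beam is a projectile actor in the defense tower game that handles its own impact effects.
; On a hit it spawns a blue beam impact emitter at the hit location and destroys itself.
; Its box overlap spawns an enlarged laser spark on any EnemyCharacter it touches, without applying damage here.
; Logic to steer the ProjectileMovement velocity toward a Target is present but never runs.
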(event `self.ReceiveHit`
  (params (MyComp :type "PrimitiveComponent Object Reference") (Other :type "Actor Object Reference") (OtherComp :type "PrimitiveComponent Object Reference") (bSelfMoved :type Boolean) (HitLocation :type "Vector Structure") (HitNormal :type "Vector Structure") (NormalImpulse :type "Vector Structure") (Hit :type "HitResult Structure (by ref)"))
  ;[1 1 1] Event hit determines spawn location for impact effect
  (`GameplayStatics.SpawnEmitterAtLocation` "/Game/BeamsAndLazers/Particles/P_BlueBeamImpact.P_BlueBeamImpact" HitLocation)
  ;[1 1 1] Destroys actor after either the projectile collides with an object or after 10 seconds
  (`self.K2_DestroyActor`))

(event `self.Box1.OnComponentBeginOverlap`
  (params (OverlappedComponent :type "PrimitiveComponent Object Reference") (OtherActor :type "Actor Object Reference") (OtherComp :type "PrimitiveComponent Object Reference") (OtherBodyIndex :type Integer) (bFromSweep :type Boolean) (SweepResult :type "HitResult Structure (by ref)"))
  (cast `/Game/Blueprints/EnemyCharacter` OtherActor)
  (`GameplayStatics.SpawnEmitterAtLocation` "/Game/StarterContent/Particles/LaserSpark.LaserSpark" (`self.K2_GetActorLocation` OtherActor) (struct) (3.0 3.0 3.0)))

(fn `UserConstructionScript`)