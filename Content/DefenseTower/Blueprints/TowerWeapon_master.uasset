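; TowerWeapon_master is a tower defense projectile actor, apparently the base for tower weapons, that explodes on contact with enemies.
; When its Box overlaps an EnemyCharacter, it spawns a Niagara explosion at its location and destroys itself, applying no damage in this graph.
; Logic to steer the ProjectileMovement velocity toward a Target is present but disconnected, so it never runs.
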(event `self.ReceiveBeginPlay`)

(event `self.Box.OnComponentBeginOverlap`
  (params (OverlappedComponent :type "PrimitiveComponent Object Reference") (OtherActor :type "Actor Object Reference") (OtherComp :type "PrimitiveComponent Object Reference") (OtherBodyIndex :type Integer) (bFromSweep :type Boolean) (SweepResult :type "HitResult Structure (by ref)"))
  (cast `/Game/Blueprints/EnemyCharacter` OtherActor)
  (`NiagaraFunctionLibrary.SpawnSystemAtLocation` "/Game/DefenseTower/Particles/NigS_TB_exp_1.NigS_TB_exp_1" (`self.K2_GetActorLocation`))
  (`self.K2_DestroyActor`))

(fn `UserConstructionScript`)