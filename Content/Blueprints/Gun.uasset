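; Gun is a weapon actor Blueprint that fires bullets automatically while its trigger is held.
; PullTriger fires once immediately through a DoOnce, then starts a looping timer on Fire at the RoundsPerSecond rate.
; ReleaseTriger clears the timer and resets the DoOnce.
; Each Fire spawns a Bullet at every Arrow component's world transform, so the arrows act as muzzles.
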(event `PullTriger`
  (`/Engine/EditorBlueprintResources/StandardMacros.DoOnce` false :!label _label
    (:`Completed`
      (`self.Fire`)
      (`KismetSystemLibrary.K2_SetTimer` null "Fire" (/ 1.0 (`self.RoundsPerSecond`)) true))))

(event `ReleaseTriger`
  (`KismetSystemLibrary.K2_ClearTimer` null "Fire")
  (goto _label :!via `Reset`))

(event `Fire`
  (for _array_element (`self.K2_GetComponentsByClass` "/Script/Engine.ArrowComponent")
    (`|SpawnActorFromClass` (`self.Bullet`) (`SceneComponent.K2_GetComponentToWorld` _array_element) "Undefined" "OverrideRootScale" null null)))

(fn `UserConstructionScript`)