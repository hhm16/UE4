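; Base enemy character that handles health, death and a day/night behavior state.
; On BeginPlay it reads the SunLight actor's Day flag to call BeNormal or BeCrazy, then gathers SpawnerType actors without using the result.
; AffectHealth applies a delta through CalculateHealth, which flags death below zero.
; Death makes the capsule ignore Pawn and WorldDynamic, detaches the controller and starts a delay with no follow-up action.
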(event `self.ReceiveBeginPlay`
  (bind _returnvalue (`GameplayStatics.GetActorOfClass` "/Game/Blueprints/SunLight.SunLight_C"))
  (if (`/Game/Blueprints/SunLight.Day` _returnvalue)
    (`self.BeNormal`)
    (else
      (`self.BeCrazy`)))
  (`GameplayStatics.GetAllActorsOfClass` (`self.SpawnerType`)))

(event `CalculateHealth`
  (params (Delta :type "Float (double-precision)"))
  (bind _output_get (set `self.Health` (+ (`self.Health`) Delta)))
  (if (< _output_get 0.0)
    (set `self.IsDead` true)))

(event `/Game/Blueprints/iDamageable.Affect Health`
  (params (Delta :type "Float (single-precision)"))
  (`self.CalculateHealth` Delta)
  (if (`self.isDead`)
    (`PrimitiveComponent.SetCollisionResponseToChannel` (`self.CapsuleComponent`) "ECC_WorldDynamic" "ECR_Ignore")
    (`PrimitiveComponent.SetCollisionResponseToChannel` (`self.CapsuleComponent`) "ECC_Pawn" "ECR_Ignore")
    (`self.DetachFromControllerPendingDestroy`)
    (`KismetSystemLibrary.Delay` 3.0)))

(fn `UserConstructionScript`)