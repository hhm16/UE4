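; Sun light actor that drives the day/night cycle and switches enemy behavior with it.
; Tick rotates it by a fixed step per frame, unscaled by delta time, and treats negative pitch as day, otherwise night.
; Two DoOnce gates reset each other so each transition fires once, printing a message and setting Day while looping over EnemyCharacter and EnemyBaseCharacterBP actors to calm them by day or enrage them at night.
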(event `self.ReceiveBeginPlay`
  (`self.K2_SetActorRotation` (struct :`Pitch` -180.0)))

(event `self.ReceiveTick`
  (params (DeltaSeconds :type "Float (single-precision)"))
  (bind (_returnvalue_roll _returnvalue_pitch) (`KismetMathLibrary.BreakRotator` (`self.K2_GetActorRotation`)))
  (`self.K2_AddActorLocalRotation` (struct :`Pitch` 0.1))
  (if (< _returnvalue_pitch 0.0)
    (`/Engine/EditorBlueprintResources/StandardMacros.DoOnce` false :!label _label
      (:`Completed`
        (`KismetSystemLibrary.PrintString` "白天降临")
        (`|ExecutionSequence`
          (:`then_0`
            (bind _outactors (`GameplayStatics.GetAllActorsOfClass` "/Game/Blueprints/EnemyCharacter.EnemyCharacter_C"))
            (for _array_element _outactors
              (bind _asenemy_character (cast `/Game/Blueprints/EnemyCharacter` _array_element))
              (`/Game/Blueprints/EnemyCharacter.Normal` _asenemy_character)
              (set `self.Day` true)))
          (:`then_1`
            (bind _outactors_2 (`GameplayStatics.GetAllActorsOfClass` "/Game/Blueprints/EnemyBaseCharacterBP.EnemyBaseCharacterBP_C"))
            (for _array_element_2 _outactors_2
              (bind _asenemy_base_character_bp (cast `/Game/Blueprints/EnemyBaseCharacterBP` _array_element_2))
              (`/Game/Blueprints/EnemyBaseCharacterBP.BeNormal` _asenemy_base_character_bp)
              (set `self.Day` true)))
          (:`then_2`
            (goto _label_2 :!via `Reset`)))))
    (else
      (`/Engine/EditorBlueprintResources/StandardMacros.DoOnce` false :!label _label_2
        (:`Completed`
          (`KismetSystemLibrary.PrintString` "黑夜降临")
          (`|ExecutionSequence`
            (:`then_0`
              (bind _outactors_3 (`GameplayStatics.GetAllActorsOfClass` "/Game/Blueprints/EnemyCharacter.EnemyCharacter_C"))
              (for _array_element_3 _outactors_3
                (bind _asenemy_character_2 (cast `/Game/Blueprints/EnemyCharacter` _array_element_3))
                (`/Game/Blueprints/EnemyCharacter.Crazy` _asenemy_character_2)
                (set `self.Day` false)))
            (:`then_1`
              (bind _outactors_4 (`GameplayStatics.GetAllActorsOfClass` "/Game/Blueprints/EnemyBaseCharacterBP.EnemyBaseCharacterBP_C"))
              (for _array_element_4 _outactors_4
                (bind _asenemy_base_character_bp_2 (cast `/Game/Blueprints/EnemyBaseCharacterBP` _array_element_4))
                (`/Game/Blueprints/EnemyBaseCharacterBP.BeCrazy` _asenemy_base_character_bp_2)
                (set `self.Day` false)))
            (:`then_2`
              (goto _label :!via `Reset`))))))))

(fn `UserConstructionScript`)