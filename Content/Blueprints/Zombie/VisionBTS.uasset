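; Behavior tree service that gives zombie AI a simple vision check for spotting the player.
; Each tick it compares the pawn's forward vector with the direction to player pawn 0 using a dot product and arccosine.
; Within a 55-degree half-angle, it writes the player to the HeroCharacter blackboard key and prints its name.
; It has no distance or line-of-sight test and never clears the key.
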(event `self.ReceiveTickAI`
  (params (OwnerController :type "AIController Object Reference") (ControlledPawn :type "Pawn Object Reference") (DeltaSeconds :type "Float (single-precision)"))
  (bind _herocharacter (`self.HeroCharacter`))
  (if (< (`KismetMathLibrary.DegAcos` (`KismetMathLibrary.Dot_VectorVector` (`KismetMathLibrary.Normal` (- (`Actor.K2_GetActorLocation` (`GameplayStatics.GetPlayerPawn` 0)) (`Actor.K2_GetActorLocation` ControlledPawn))) (`Actor.GetActorForwardVector` ControlledPawn))) 55.0)
    (`BTFunctionLibrary.SetBlackboardValueAsObject` _herocharacter (`GameplayStatics.GetPlayerPawn` 0))
    (`KismetSystemLibrary.PrintString` (`KismetSystemLibrary.GetDisplayName` (`BTFunctionLibrary.GetBlackboardValueAsObject` _herocharacter)))))