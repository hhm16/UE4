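; Wall actor that destroys any Projectile overlapping it and adapts its cube materials to its size.
; On BeginPlay it creates dynamic instances for both material slots, side and up, with BrickMat as the source for the latter.
; Each instance receives a Zoom vector from the cube's world X and Y scale, with the axes swapped between them, apparently to keep texture tiling proportional.
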(event `self.ReceiveBeginPlay`
  (bind _cube (`self.Cube`))
  (bind (_returnvalue_x _returnvalue_y) (`KismetMathLibrary.BreakVector` (`SceneComponent.K2_GetComponentScale` _cube)))
  (`|ExecutionSequence`
    (:`then_0`
      (bind _returnvalue (`PrimitiveComponent.CreateDynamicMaterialInstance` _cube 0 null "None"))
      (bind _output_get (set `self.MateralSide` _returnvalue))
      (`MaterialInstanceDynamic.SetVectorParameterValue` _output_get "Zoom" (make `LinearColor` _returnvalue_y _returnvalue_x 0.0 1.0)))
    (:`then_1`
      (bind _returnvalue_2 (`PrimitiveComponent.CreateDynamicMaterialInstance` _cube 1 "/Game/Materials/BrickMat.BrickMat" "None"))
      (bind _output_get_2 (set `self.MateralUp` _returnvalue_2))
      (`MaterialInstanceDynamic.SetVectorParameterValue` _output_get_2 "Zoom" (make `LinearColor` _returnvalue_x _returnvalue_y 1.0 1.0)))))

(event `self.ReceiveActorBeginOverlap`
  (params (OtherActor :type "Actor Object Reference"))
  (bind _asprojectile (cast `/Game/Blueprints/Projectile` OtherActor))
  (`self.K2_DestroyActor` _asprojectile))

(fn `UserConstructionScript`)