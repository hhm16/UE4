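; DistanceBTS is a behavior tree service that decides whether a zombie enemy chases the player.
; Each tick it compares the distance between the controlled EnemyBaseCharacterBP and player pawn 0 against that enemy's SearchRange.
; It writes the matching zombie state (chase or stop chasing) and the current distance to the Blackboard.
; Debug strings print on every tick and for each branch.
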(event `self.ReceiveTickAI`
  (params (OwnerController :type "AIController Object Reference") (ControlledPawn :type "Pawn Object Reference") (DeltaSeconds :type "Float (single-precision)"))
  (bind _state (`self.State`))
  (bind _returnvalue (`KismetMathLibrary.VSize` (- (`Actor.K2_GetActorLocation` (`GameplayStatics.GetPlayerPawn` 0)) (`Actor.K2_GetActorLocation` ControlledPawn))))
  ;[1 1 1] 获取位置
  (`KismetSystemLibrary.PrintString` "你好")
  (bind _asenemy_base_character_bp (cast `/Game/Blueprints/EnemyBaseCharacterBP` ControlledPawn))
  (if (< _returnvalue (`/Game/Blueprints/EnemyBaseCharacterBP.SearchRange` _asenemy_base_character_bp))
    (`KismetSystemLibrary.PrintString` "开始追逐")
    (`BTFunctionLibrary.SetBlackboardValueAsEnum` _state (enumliteral `/Game/Blueprints/ZombieState` "NewEnumerator1"))
    (`BTFunctionLibrary.SetBlackboardValueAsFloat` (`self.Distance`) _returnvalue)
    (else
      (`KismetSystemLibrary.PrintString` "停止追逐")
      (`BTFunctionLibrary.SetBlackboardValueAsEnum` _state (enumliteral `/Game/Blueprints/ZombieState` "NewEnumerator0"))
      (`BTFunctionLibrary.SetBlackboardValueAsFloat` (`self.Distance`) _returnvalue))))